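; AI controller for a CPU prisoner that the player can rescue.
; On begin play it runs the BTPrisoner behavior tree and stores the player pawn as the TargetActor blackboard key.
; Any AI perception update sets IsRescued to true and prints a debug message, without checking the sensed actor or stimulus.
; Each tick writes the pawn's distance to the player into DistanceToPlayer for the tree.
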(event `self.ReceiveBeginPlay`
  (`self.RunBehaviorTree` "/Game/CPU/BTPrisoner.BTPrisoner")
  (`BlackboardComponent.SetValueAsObject` (`AIBlueprintHelperLibrary.GetBlackboard` null) "TargetActor" (`GameplayStatics.GetPlayerPawn` 0)))

(event `self.AIPerception.OnTargetPerceptionUpdated`
  (params (Actor :type "Actor Object Reference") (Stimulus :type "AIStimulus Structure"))
  (`BlackboardComponent.SetValueAsBool` (`AIBlueprintHelperLibrary.GetBlackboard` null) "IsRescued" true)
  (`KismetSystemLibrary.PrintString` "Rescued!"))

(event `self.ReceiveTick`
  (params (DeltaSeconds :type "Float (single-precision)"))
  (`BlackboardComponent.SetValueAsFloat` (`AIBlueprintHelperLibrary.GetBlackboard` null) "DistanceToPlayer" (`self.GetDistanceTo` (`self.K2_GetPawn`) (`GameplayStatics.GetPlayerPawn` 0))))

(fn `UserConstructionScript`)