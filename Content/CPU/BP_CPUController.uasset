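; BP_CPUController is an AI controller that runs the BTGuard behavior tree for a guard pawn and supplies its blackboard.
; On BeginPlay it stores the pawn's starting location as GuardPos.
; AI perception updates write the reported actor to TargetActor, without checking whether it was sensed or lost.
; While that target is valid, Tick writes its distance from the pawn to DistanceToPlayer.
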(event `self.ReceiveBeginPlay`
  (`self.RunBehaviorTree` "/Game/CPU/BTGuard.BTGuard")
  (`BlackboardComponent.SetValueAsVector` (`AIBlueprintHelperLibrary.GetBlackboard` null) "GuardPos" (`self.K2_GetActorLocation` (`self.K2_GetPawn`))))

(event `self.AIPerception.OnTargetPerceptionUpdated`
  (params (Actor :type "Actor Object Reference") (Stimulus :type "AIStimulus Structure"))
  (`BlackboardComponent.SetValueAsObject` (`AIBlueprintHelperLibrary.GetBlackboard` null) (`self.TargetActor`) Actor))

(event `self.ReceiveTick`
  (params (DeltaSeconds :type "Float (single-precision)"))
  (bind _returnvalue (`BlackboardComponent.GetValueAsObject` (`AIBlueprintHelperLibrary.GetBlackboard` null) "TargetActor"))
  (if (`KismetSystemLibrary.IsValid` _returnvalue)
    (bind _asactor (cast `Actor` _returnvalue))
    (`BlackboardComponent.SetValueAsFloat` (`AIBlueprintHelperLibrary.GetBlackboard` null) "DistanceToPlayer" (`self.GetDistanceTo` _asactor (`self.K2_GetPawn`)))))

(fn `UserConstructionScript`)